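; PatrolRouteBase is an actor that defines an AI guard patrol route as an array of patrol points.
; Its construction script flushes persistent debug lines, then transforms each point from the actor's local space to world space.
; It draws thick, timed blue debug lines between consecutive points to show the route, leaving the loop open.
; The event graph holds no active logic.
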(event EventBeginPlay)

(event Collision|EventActorBeginOverlap
  (params (OtherActor :type Actor%20Object%20Reference)))

(event EventTick
  (params (DeltaSeconds :type Float%20%28single-precision%29)))

(fn ConstructionScript
  (bind _returnvalue (Transformation|GetActorTransform))
  ;[1 1 1] Draws a line between point to show guard route
  (Rendering|Debug|FlushPersistentDebugLines)
  (for (_array_element _array_index) (Variables|Default|GetPatrolPoints)
    (if (!= _array_index 0)
      (Rendering|Debug|DrawDebugLine (Math|Transform|TransformLocation _returnvalue _array_element) (Math|Transform|TransformLocation _returnvalue (Utilities|Array|Get(acopy) (Variables|Default|GetPatrolPoints) (- _array_index 1))) "(R=0.038182,G=0.126636,B=0.796875,A=1.000000)" 1e+01 5e+01))))